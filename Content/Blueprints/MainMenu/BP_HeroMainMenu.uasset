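; BP_HeroMainMenu is the main menu scene actor that starts the menu and animates a fireball and magic circle.
; On BeginPlay it plays menu music, adds WBP_MainMenu to the viewport, switches input to UI-only and shows the cursor.
; Tick bobs the fireball vertically around its starting world location with a sine of accumulated time, and spins the magic circle decal about its roll axis at a configurable rate.
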(event EventBeginPlay
  (Variables|Default|SetFireballInitialLocation (Transformation|GetWorldLocation (Variables|Default|GetFireBall)))
  (Audio|PlaySound2D "/Game/Assets/Sounds/Music/Music_MainMenu.Music_MainMenu" 1.0 1.0 0.0 0 0)
  (bind _returnvalue (UserInterface|CreateWidget "/Game/Blueprints/MainMenu/WBP_MainMenu.WBP_MainMenu_C"))
  (UserInterface|Viewport|AddtoViewport _returnvalue 0)
  (Input|SetInputModeUIOnly (Game|GetPlayerController 0) _returnvalue "DoNotLock" false) ; 设置只允许此UI响应用户的输入操作
  (Variables|/Script/Engine.PlayerController|SetbShowMouseCursor (Game|GetPlayerController 0) true) ; 设置显示鼠标光标
)

(event Collision|EventActorBeginOverlap
  (params (OtherActor :type Actor%20Object%20Reference)))

(event EventTick
  (params (DeltaSeconds :type Float%20%28single-precision%29))
  (bind _output_get (Variables|Default|SetDelta%20Seconds DeltaSeconds))
  (bind _output_get_2 (Variables|Default|SetTime (+ _output_get (Variables|Default|GetTime))))
  (Transformation|SetWorldLocation (Variables|Default|GetFireBall) (+ (Variables|Default|GetFireballInitialLocation) (Math|Vector|MakeVector 0.0 0.0 (* (Math|Trig|Sin(Radians) _output_get_2) (Variables|Default|GetAmplitude)))) false false) ; 让火球浮动
  (Transformation|AddLocalRotation (Variables|Default|GetMagicCircleDecal) (Math|Rotator|MakeRotator (* (Variables|Default|GetDelta%20Seconds) (Variables|Default|GetMagicCircleRotationRate)) 0.0 0.0) false false) ; 让头后面的魔法光环旋转起来
)

(fn ConstructionScript)