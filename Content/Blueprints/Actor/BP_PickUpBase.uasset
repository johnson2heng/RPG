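; Base pickup actor that animates its spawn, then rotates and bobs, with sounds for spawn, ground impact and destruction.
; A timeline drives height and scale on spawn, firing the impact sound once when elevation is near zero.
; When it finishes, it starts rotation and sinusoidal movement through functions defined outside these graphs.
; Tick applies the calculated location and rotation to the actor every frame.
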(event EventBeginPlay
  (Audio|PlaySoundatLocation (Variables|Default|GetSpawnSound) (Transformation|GetActorLocation) "0, 0, 0" 1.0 1.0 0.0 0 0 0 0) ; 播放生成音效
  (bind (_direction _elevation _scale) (Timeline|PickupElevationTimeline Play)
    (:Update
      (CallFunction|UpdateLocationandScale _elevation _scale) ; 时间轴更新位置和缩放
      (if (< _elevation 0.1) ; 大于0.8s播放一次音效
        (Utilities|FlowControl|DoOnce false
          (:Completed
            (Audio|PlaySoundatLocation (Variables|Default|GetGroundImpactSound) (Transformation|GetActorLocation) "0, 0, 0" 1.0 1.0 0.0 0 0 0 0)))))
    (:Finished
      ;[1 1 1] 时间轴结束开始自动模式
      (Class|RPGEffectActor|StartRotation) ; 开始旋转
      (Class|RPGEffectActor|StartSinusoidalMovement) ; 开始移动
    )))

(event Collision|EventActorBeginOverlap
  (params (OtherActor :type Actor%20Object%20Reference)))

(event EventTick
  (params (DeltaSeconds :type Float%20%28single-precision%29))
  (Transformation|SetActorLocation (Variables|Default|GetCalculatedLocation) false false) ; 更新位置
  (Transformation|SetActorRotation (Variables|Default|GetCalculatedRotation)) ; 更新转向
)

(event EventDestroyed
  (Audio|PlaySoundatLocation (Variables|Default|GetConsumedSound) (Transformation|GetActorLocation) "0, 0, 0" 1.0 1.0 0.0 0 0 0 0) ; 播放拾取音效
)

(fn ConstructionScript)

(fn UpdateLocationandScale
  (params (Elevation :type Float%20%28single-precision%29) (Scale :type Float%20%28single-precision%29))
  (bind _calculatedlocation (Variables|Default|GetCalculatedLocation))
  (Transformation|SetActorLocation (Math|Vector|MakeVector (.x _calculatedlocation) (.y _calculatedlocation) (+ (.z _calculatedlocation) (* Elevation (Variables|Default|GetSpawnApex)))) false false)
  (Transformation|SetActorScale3D (Math|Vector|MakeVector Scale Scale Scale)) ; 更新缩放
)