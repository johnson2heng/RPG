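; Enemy melee attack gameplay ability that turns the avatar toward its combat target and plays a random tagged attack montage.
; When the montage's tagged gameplay event arrives, it gathers live players in a small sphere around the montage's combat socket.
; Non-friendly targets take damage and trigger a hit-effect cue, and any hit also plays an impact-sound cue keyed by the montage tag.
; The ability ends when the montage finishes or is interrupted.
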(event Ability|EventActivateAbility
  (bind _returnvalue (Ability|GetAvatarActorfromActorInfo))
  (bind _returnvalue_2 (Ability|GetAvatarActorfromActorInfo))
  ;[1 1 1] 通过战斗接口获取攻击目标，并通过motionwrapping更新朝向
  (Variables|Default|SetHasHitTarget false)
  (bind _ascombat_interface (Utilities|Casting|CastToCombatInterface _returnvalue)
    (:then
      (Variables|Default|SetCombat%20Interface _ascombat_interface)
      (bind _returnvalue_3 (Class|EnemyInterface|GetCombatTarget(Message) _returnvalue))
      (Class|CombatInterface|UpdateFacingTarget (Variables|Default|GetCombat%20Interface) (Transformation|GetActorLocation _returnvalue_3))
      ;[1 1 1] 从攻击动作中获取一套攻击，播放动作等待触发伤害事件
      (bind _returnvalue_4 (Class|CombatInterface|GetAttackMontages(Message) (Ability|GetAvatarActorfromActorInfo)))
      (bind _output_get (Variables|Default|SetMontageStruct (Class|RPGDamageGameplayAbility|GetRandomTaggedMontagefromArray _returnvalue_4))) ; 保存变量
      (|PlayMontageandWaitProxy "None" (.Montage (Utilities|Struct|BreakTaggedMontage _output_get)) 1.0 "None" true 1.0 0.0 false
        (:then
          (Ability|Tasks|WaitGameplayEvent (.SocketTag (Utilities|Struct|BreakTaggedMontage _output_get)) 0
            (:EventReceived
              ;[1 1 1] 通过骨骼获取伤害位置，并通过位置获取到范围内的所有Actor
              (bind _output_get_2 (Variables|Default|SetCombatLocation (Class|CombatInterface|GetCombatSocketLocationbyStruct (Variables|Default|GetCombat%20Interface) (Variables|Default|GetMontageStruct))))
              (bind _outoverlappingactors (Class|RPGAbilitySystemLibrary|GetLivePlayersWithinRadius _returnvalue_2 (Utilities|Array|MakeArray _returnvalue_2) 45.0 _output_get_2))
              ;[1 1 1] 遍历所有范围内的Actor，如果是敌对单位，将应用伤害GE，并播放伤害表现效果
              (for _array_element _outoverlappingactors
                (bind _output_get_3 (Variables|Default|SetForEachActor _array_element))
                (if (Class|RPGAbilitySystemLibrary|IsNotFriend _output_get_3 (Ability|GetAvatarActorfromActorInfo))
                  (Class|RPGDamageGameplayAbility|CauseDamage (Variables|Default|GetForEachActor))
                  (Variables|Default|SetHasHitTarget true)
                  (Class|GameplayAbility|ExecuteGameplayCuewithParams "(TagName=\"GameplayCue.HitEffect\")" (Ability|GameplayCue|MakeGameplayCueParameters :Location (Transformation|GetActorLocation (Variables|Default|GetForEachActor)) :SourceObject (Variables|Default|GetForEachActor)))))
              ;[1 1 1] 遍历完成后如果击中敌人，将播放击中音效
              (if (Variables|Default|GetHasHitTarget) ; 击中敌人播放音效
                (Class|GameplayAbility|ExecuteGameplayCuewithParams "(TagName=\"GameplayCue.ImpactSound\")" (Ability|GameplayCue|MakeGameplayCueParameters :AggregatedSourceTags (GameplayTags|MakeGameplayTagContainerfromTag (.MontageTag (Utilities|Struct|BreakTaggedMontage (Variables|Default|GetMontageStruct)))) :Location (Variables|Default|GetCombatLocation) :EffectCauser (Ability|GetAvatarActorfromActorInfo)))))))
        (:OnCompleted
          (Ability|EndAbility :!label _label) ; 动画播放完成，或中断，直接停止此技能
        )
        (:OnBlendOut
          (goto _label))
        (:OnInterrupted
          (goto _label))
        (:OnCancelled
          (goto _label))))
    (:CastFailed
      (Ability|EndAbility))))