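; Enemy summon ability that spawns random minions at shuffled spawn locations around the caster.
; It plays ground-summon Niagara effects at each point and the Shaman summon montage, waiting for a weapon socket gameplay event.
; On that event it spawns AI-controlled minions one by one with a short delay, facing away from the caster.
; Each spawn increments the caster's minion count, decremented again when that minion is destroyed.
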(event Custom|OnDestroyed_事件
  (params (DestroyedActor :type Actor%20Object%20Reference))
  (Class|CombatInterface|IncrementMinionCount(Message) (Ability|GetAvatarActorfromActorInfo) -1) ; 减少仆从
)

(event Ability|EventActivateAbility
  (bind _returnvalue (Class|RPGSummonAbility|GetSpawnLocations))
  (bind _output_get (Variables|Default|SetSpawnLocations _returnvalue))
  (Utilities|Array|Shuffle _output_get)
  (Utilities|FlowControl|Sequence
    (:then_0
      (for _array_element (Variables|Default|GetSpawnLocations)
        (Niagara|SpawnSystematLocation "/Game/Assets/Effects/Combat/NS_GroundSummon.NS_GroundSummon" _array_element "0, 0, 0" "1.000000,1.000000,1.000000" true true "AutoRelease") ; 在目标位置生成粒子特效
      ))
    (:then_1
      (|PlayMontageandWaitProxy "None" "/Game/Assets/Enemies/Shaman/Animations/AM_Shaman_Summon.AM_Shaman_Summon" 1.0 "None" true 1.0 0.0 false
        (:then
          (Ability|Tasks|WaitGameplayEvent "(TagName=\"CombatSocket.Weapon\")" 0
            (:EventReceived
              (Variables|Default|SetSpawnLocationsIndex 0)
              (if (< (Variables|Default|GetSpawnLocationsIndex) (Utilities|Array|Length (Variables|Default|GetSpawnLocations))) :!label _label
                (bind _returnvalue_2 (Game|SpawnActorfromClass (Class|RPGSummonAbility|GetRandomMinionClass) (Math|Transform|MakeTransform (+ (Utilities|Array|Get(acopy) (Variables|Default|GetSpawnLocations) (Variables|Default|GetSpawnLocationsIndex)) "0.000000,0.000000,70.000000") (Math|Rotator|FindLookatRotation (Transformation|GetActorLocation (Ability|GetAvatarActorfromActorInfo)) (Utilities|Array|Get(acopy) (Variables|Default|GetSpawnLocations) (Variables|Default|GetSpawnLocationsIndex))) "1.000000,1.000000,1.000000") "AdjustIfPossibleButAlwaysSpawn" "MultiplyWithRoot" 0 0))
                (Pawn|SpawnDefaultController _returnvalue_2)
                (Game|AssignOnDestroyed _returnvalue_2 (delegate Custom|OnDestroyed_事件))
                (Class|CombatInterface|IncrementMinionCount(Message) (Ability|GetAvatarActorfromActorInfo) 1) ; 增加仆从
                (Math|Integer|IncrementInt (Variables|Default|GetSpawnLocationsIndex)
                  (:%20%20
                    (Utilities|FlowControl|Delay 0.1)
                    (goto _label)))))))
        (:OnCompleted
          (Ability|EndAbility :!label _label_2))
        (:OnBlendOut
          (goto _label_2))
        (:OnCancelled
          (goto _label_2))))))