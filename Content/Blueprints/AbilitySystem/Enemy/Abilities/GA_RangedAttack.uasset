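; GA_RangedAttack is an enemy gameplay ability that performs a ranged attack on the avatar's current combat target.
; It turns the avatar toward the target and plays a montage picked at random from the avatar's tagged attack montages.
; When the gameplay event matching the montage's socket tag arrives, it re-reads the target's location and spawns a projectile from that socket toward it.
; The ability ends when the montage completes, blends out or is cancelled.
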(event Ability|EventActivateAbility
  (bind _returnvalue (Ability|GetAvatarActorfromActorInfo))
  (bind _returnvalue_2 (Class|EnemyInterface|GetCombatTarget(Message) _returnvalue)) ; 获取攻击目标
  (Class|CombatInterface|UpdateFacingTarget(Message) _returnvalue (Transformation|GetActorLocation _returnvalue_2)) ; 朝向目标
  (bind _returnvalue_3 (Class|CombatInterface|GetAttackMontages(Message) (Ability|GetAvatarActorfromActorInfo))) ; 获取角色所有攻击动画
  (bind _output_get (Variables|Default|SetTaggedMontage (Class|RPGDamageGameplayAbility|GetRandomTaggedMontagefromArray _returnvalue_3))) ; 获取随机的蒙太奇
  (|PlayMontageandWaitProxy "None" (.Montage (Utilities|Struct|BreakTaggedMontage _output_get)) 1.0 "None" true 1.0 0.0 false
    (:then
      (Ability|Tasks|WaitGameplayEvent (.SocketTag (Utilities|Struct|BreakTaggedMontage _output_get)) 0
        (:EventReceived
          (bind _returnvalue_4 (Class|EnemyInterface|GetCombatTarget(Message) (Ability|GetAvatarActorfromActorInfo))) ; 获取攻击目标
          (Class|ProjectileSpell|SpawnProjectile (Transformation|GetActorLocation _returnvalue_4) (.SocketTag (Utilities|Struct|BreakTaggedMontage (Variables|Default|GetTaggedMontage))) (.CombatTipSocketName (Utilities|Struct|BreakTaggedMontage (Variables|Default|GetTaggedMontage)))))))
    (:OnCompleted
      (Ability|EndAbility :!label _label))
    (:OnBlendOut
      (goto _label))
    (:OnCancelled
      (goto _label))))

(event Ability|EventOnEndAbility
  (params (bWasCancelled :type Boolean)))