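; Arcane Shards gameplay ability that strikes a series of points around a player-targeted location with radial damage.
; It shows a magic circle, waits for input, then takes ground points from a spawned BP_PointCollection at the cursor's impact with random yaw.
; A montage event starts a looping timer that, per point, executes a GameplayCue and damages live players in radius with upward knockback.
; Ending the ability cleans up the points, timer and circle.
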(event Custom|SpawnShard
  (bind _returnvalue (Ability|GetAvatarActorfromActorInfo))
  (bind _result (Math|Integer|IncrementInt (Variables|Default|GetIndex))
    (:%20%20
      (if (<= _result (Variables|Default|GetNum%20Points)) ; 如果索引大于生成数量，将结束技能停止定时器
        (Variables|Default|SetShardLocation (Transformation|GetWorldLocation (Utilities|Array|Get(acopy) (Variables|Default|GetGroundPoints) (- (Variables|Default|GetIndex) 1)))) ; 获取技能个体爆炸的位置
        (GameplayCue|ExecuteGameplayCueOnActor(Burst) (Ability|GetOwningActorfromActorInfo) "(TagName=\"GameplayCue.ArcaneShards\")" (Ability|GameplayCue|MakeGameplayCueParameters :Location (Variables|Default|GetShardLocation))) ; 播放技能效果
        (bind _outoverlappingactors (Class|RPGAbilitySystemLibrary|GetLivePlayersWithinRadius _returnvalue (Utilities|Array|MakeArray _returnvalue) (Variables|Default|GetRadialDamageOuterRadius) (Variables|Default|GetShardLocation))) ; 获取技能可以命中的目标
        (bind _output_get (Variables|Default|SetOut%20Overlapping%20Actors _outoverlappingactors)) ; 保存变量防止多次调用前面节点
        (for _array_element _output_get ; 遍历应用伤害
          (Class|RPGAbilitySystemLibrary|ApplyDamageEffect (Class|RPGDamageGameplayAbility|MakeDamageEffectParamsfromClassDefaults _array_element (Variables|Default|GetShardLocation) true "0.000000,0.000000,1.000000" false "0, 0, 0")) ; 使用函数库函数应用伤害
        )
        (else
          (Ability|EndAbility))))))

(event Custom|SpawnShards
  (Variables|Default|SetIndex 0)
  (bind _returnvalue (Utilities|Time|SetTimerbyEvent (delegate Custom|SpawnShard) (Variables|Default|GetShardSpawnTime) true)) ; 使用定时器循环生成个体
  (Variables|Default|SetSpawnTimerHandle _returnvalue)
  ;[1 1 1] 隐藏标识光圈，并调用一次生成事件
  (Class|PlayerInterface|HideMagicCircle(Message) (Ability|GetAvatarActorfromActorInfo)) ; 隐藏光圈
  (CallFunction|SpawnShard) ; 先调用一次事件，触发后生成一个个体
)

(event Ability|EventActivateAbility
  (Utilities|FlowControl|Sequence
    (:then_0
      (Class|PlayerInterface|ShowMagicCircle(Message) (Ability|GetAvatarActorfromActorInfo) 0) ; 显示范围标识
    )
    (:then_1
      (Ability|Tasks|WaitInputPress false ; 等待技能再次输入
        (:OnPress
          (bind _datahandle (|TargetDataUnderMouse)
            (:ValidData
              (bind _output_get (Variables|Default|SetImpact%20Point (.ImpactPoint (Collision|BreakHitResult (Ability|TargetData|GetHitResultfromTargetData _datahandle)))))
              (bind _returnvalue (Game|SpawnActorfromClass "/Game/Blueprints/AbilitySystem/Hero/Abilities/Arcane/ArcaneShards/BP_PointCollection.BP_PointCollection_C" (Math|Transform|MakeTransform _output_get "0, 0, 0" "1.000000,1.000000,1.000000") "AlwaysSpawn" "MultiplyWithRoot" 0 0)) ; 通过位置拾取actor获取一些随机生成点
              ;[1 1 1] 获取可以生成技能攻击位置的点的数组
              (bind _output_get_2 (Variables|Default|SetPointCollection _returnvalue))
              (Variables|Default|SetGroundPoints (Class|PointCollection|GetGroundPoints _output_get_2 (Variables|Default|GetImpact%20Point) (Variables|Default|GetNum%20Points) (Math|Random|RandomFloatinRange 0.0 3.6e+02)))
              ;[1 1 1] 切换朝向和播放动作监听通知
              (Class|CombatInterface|UpdateFacingTarget(Message) (Ability|GetAvatarActorfromActorInfo) (Variables|Default|GetImpact%20Point))
              (|PlayMontageandWaitProxy "None" "/Game/Assets/Characters/Aura/Animations/Abilities/AM_Cast_ArcaneShards.AM_Cast_ArcaneShards" 1.0 "None" true 1.0 0.0 false
                (:then
                  (Ability|Tasks|WaitGameplayEvent "(TagName=\"Event.Montage.ArcaneShards\")" 0
                    (:EventReceived
                      (CallFunction|SpawnShards) ; 生成所有的技能个体
                    )))))))))))

(event Ability|EventOnEndAbility
  (params (bWasCancelled :type Boolean))
  (bind _pointcollection (Variables|Default|GetPointCollection)
    (:then
      (Actor|DestroyActor _pointcollection)
      (Utilities|Time|ClearandInvalidateTimerbyHandle (Variables|Default|GetSpawnTimerHandle))
      (Class|PlayerInterface|HideMagicCircle(Message) (Ability|GetAvatarActorfromActorInfo)) ; 隐藏光圈
    )
    (:else)))