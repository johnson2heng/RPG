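; BP_FireBlast is a projectile actor for the hero's FireBlast ability that flies outward, then boomerangs back to its caster.
; On authority, StartOutgoingTimeline lerps it forward to an apex at TravelDistance using a timeline.
; A second timeline then lerps it toward the live location of ReturnToActor, without sweeping.
; Within ExplodeDistance of that actor it is destroyed; the commented explosion has no logic in this graph.
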(event EventBeginPlay)

(event Collision|EventActorBeginOverlap
  (params (OtherActor :type Actor%20Object%20Reference)))

(event EventTick
  (params (DeltaSeconds :type Float%20%28single-precision%29)))

(event EventStartOutgoingTimeline
  (Networking|SwitchHasAuthority
    (:Authority
      (Variables|Default|SetInitialLocation (Transformation|GetActorLocation)) ; 初始位置
      (Variables|Default|SetApexLocation (+ (Variables|Default|GetInitialLocation) (* (Transformation|GetActorForwardVector) (Variables|Default|GetTravelDistance)))) ; 终点位置
      (bind _outgoingtrack (Timeline|OutgoingTimeline Play) ; 火球向外扩散
        (:Update
          (Transformation|SetActorLocation (Math|Vector|Lerp(Vector) (Variables|Default|GetInitialLocation) (Variables|Default|GetApexLocation) _outgoingtrack) false false))
        (:Finished
          (bind _returningtrack (Timeline|ReturningTimeline Play) ; 火球返回角色
            (:Update
              (Variables|Default|SetOwnerLocation (Transformation|GetActorLocation (Variables|Default|GetReturnToActor))) ; 技能释放者的位置
              (Transformation|SetActorLocation (Math|Vector|Lerp(Vector) (Variables|Default|GetApexLocation) (Variables|Default|GetOwnerLocation) _returningtrack) false false)
              (if (<= (Math|Vector|Distance(Vector) (Transformation|GetActorLocation) (Variables|Default|GetOwnerLocation)) (Variables|Default|GetExplodeDistance)) ; 返回时，距离玩家一定距离产生爆炸
                (Actor|DestroyActor)))))))))

(fn ConstructionScript)