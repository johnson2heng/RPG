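; BP_FireBolt is the Fire Bolt projectile actor for the hero's fire ability.
; Each Tick it stores its previous and current location and measures the distance moved that frame.
; It destroys itself when that distance is at or below MinDistancePerFrame, cleaning up a bolt that has stalled or is hovering in place.
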(event EventBeginPlay)

(event Collision|EventActorBeginOverlap
  (params (OtherActor :type Actor%20Object%20Reference)))

(event EventTick
  (params (DeltaSeconds :type Float%20%28single-precision%29))
  ;[1 1 1] 如果火球悬停后，没有移动，将其销毁，通过移动距离判断
  (Variables|Default|SetLocationLastFrame (Variables|Default|GetLocationThisFrame))
  (Variables|Default|SetLocationThisFrame (Transformation|GetActorLocation))
  (if (<= (Math|Vector|VectorLength (- (Variables|Default|GetLocationThisFrame) (Variables|Default|GetLocationLastFrame))) (Variables|Default|GetMinDistancePerFrame)) ; 如果此帧移动小于设定的最小，将销毁抛射物
    (Actor|DestroyActor)))

(fn ConstructionScript)