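; GA_Electrocute is the hero's channeled lightning ability, currently handling targeting, casting animation and movement lock, with no damage logic.
; On activation it commits, stores the cursor hit via TargetDataUnderMouse, hides the cursor, faces the target and plays the Electrocute montage.
; The montage's gameplay event starts the shock loop through an avatar interface message and disables movement.
; Releasing input restores cursor and walking, stops the loop and ends the ability.
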(event Ability|EventActivateAbility
  (CallFunction|EnforceImplementsCombatInterface) ; 确保角色已经实现战斗接口
  (Ability|CommitAbility)
  ;[1 1 1] 存储鼠标拾取数据
  (bind _datahandle (|TargetDataUnderMouse) ; 拾取攻击位置，获取攻击目标
    (:ValidData
      (Class|RPGBeamSpell|StoreMouseDataInfo (Ability|TargetData|GetHitResultfromTargetData _datahandle))
      (Class|RPGBeamSpell|StoreOwnerVariables)
      ;[1 1 1] 释放技能隐藏光标
      (Utilities|FlowControl|Sequence
        (:then_0
          (Variables|/Script/Engine.PlayerController|SetbShowMouseCursor (Variables|Default|GetOwnerPlayerController) false) ; 隐藏鼠标光标
          ;[1 1 1] 修改朝向目标，并在播放蒙太奇时转向目标
          (Class|CombatInterface|UpdateFacingTarget(Message) (Ability|GetAvatarActorfromActorInfo) (Variables|Default|GetMouseHitLocation)) ; 转向目标
          (|PlayMontageandWaitProxy "None" (Variables|Default|GetMontage_Electrocute) 1.0 "None" false 1.0 0.0 false
            (:then
              (Ability|Tasks|WaitGameplayEvent "(TagName=\"Event.Montage.Electrocute\")" 0
                (:EventReceived
                  (CallFunction|InShockLoop))))))
        (:then_1
          (Ability|Tasks|WaitInputRelease false
            (:OnRelease
              (CallFunction|PreparetoEndAbility) ; 处理技能结束前的逻辑
              (Ability|EndAbility))))))))

(fn EnforceImplementsCombatInterface
  (if (not (Utilities|DoesObjectImplementInterface (Ability|GetAvatarActorfromActorInfo) "/Script/RPG.CombatInterface"))
    (Ability|EndAbility)))

(fn PreparetoEndAbility
  (Variables|/Script/Engine.PlayerController|SetbShowMouseCursor (Variables|Default|GetOwnerPlayerController) true) ; 显示鼠标光标
  (Class|CombatInterface|SetinShockLoop(Message) (Ability|GetAvatarActorfromActorInfo) false) ; 关闭持续施法
  (Pawn|Components|CharacterMovement|SetMovementMode (Variables|/Script/Engine.Character|GetCharacterMovement (Variables|Default|GetOwnerCharacter)) "MOVE_Walking" 0) ; 恢复可移动状态
)

(fn InShockLoop
  (Class|CombatInterface|SetinShockLoop(Message) (Ability|GetAvatarActorfromActorInfo) true) ; 开启持续施法
  (Pawn|Components|CharacterMovement|DisableMovement (Variables|/Script/Engine.Character|GetCharacterMovement (Variables|Default|GetOwnerCharacter))) ; 施法时，禁止角色移动
)