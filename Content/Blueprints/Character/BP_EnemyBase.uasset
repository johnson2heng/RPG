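; Base enemy Blueprint handling spawn scale-in, motion-warped attack facing, death dissolve and loot drops.
; SpawnLoot pulls items from loot tiers, then a looping timer spawns them one by one in an evenly spaced ring at random distances.
; Flagged RPGEffectActor drops take their level from GetPlayerLevel.
; Timelines animate mesh scale on BeginPlay and the Dissolve parameter on supplied dynamic materials.
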(event Custom|SpawnLootItem
  (bind _lootitems (Variables|Default|GetLootItems))
  (bind _spawnlootcount (Variables|Default|GetSpawnLootCount))
  (bind _output (Utilities|Array|Get(acopy) _lootitems _spawnlootcount))
  (bind (_lootclass _blootleveloverride) (Utilities|Struct|BreakLootItem _output))
  (bind _returnvalue (Game|SpawnActorfromClass _lootclass (CallFunction|GetLootTransform (Variables|Default|GetSpawnLootCount)) "AdjustIfPossibleButAlwaysSpawn" "MultiplyWithRoot" 0 0)) ; 生成战利品
  (CallFunction|UpdateLootLevel _returnvalue _blootleveloverride) ; 更新等级
  (bind _result (Math|Integer|IncrementInt (Variables|Default|GetSpawnLootCount)) ; 切换索引
    (:%20%20
      (if (>= _result (Utilities|Array|Length (Variables|Default|GetLootItems))) ; 索引超过长度，清除定时器
        (Utilities|Time|ClearandInvalidateTimerbyHandle (Variables|Default|GetLootTimer))))))

(event EventBeginPlay
  (bind _scaletrack (Timeline|SpawnTimeline Play)
    (:Update
      (Transformation|SetRelativeScale3D (Variables|Character|GetMesh) (Math|Vector|MakeVector _scaletrack _scaletrack _scaletrack)))))

(event Collision|EventActorBeginOverlap
  (params (OtherActor :type Actor%20Object%20Reference)))

(event EventTick
  (params (DeltaSeconds :type Float%20%28single-precision%29)))

(event EventStartDissolveTimeline
  (params (DynamicMaterialInstance :type Array%20of%20Material%20Instance%20Dynamic%20Object%20References))
  (bind _dissolvetrack (Timeline|DissolveTimeline PlayFromStart)
    (:Update
      (for _array_element DynamicMaterialInstance
        (Rendering|Material|SetScalarParameterValue _array_element "Dissolve" _dissolvetrack :!class /Script/Engine.MaterialInstanceDynamic)))))

(event EventUpdateFacingTarget
  (params (Target :type Vector%20%28by%20ref%29 :default "0, 0, 0"))
  (Class|MotionWarpingComponent|AddorUpdateWarpTargetfromLocation (Variables|Default|GetMotionWarping) "FacingTarget" Target))

(event EventSpawnLoot
  (bind _returnvalue (Class|RPGAbilitySystemLibrary|GetLootTiers))
  (Utilities|IsValid _returnvalue
    (:Is%20Valid
      (bind _returnvalue_2 (Class|LootTiers|GetLootItems _returnvalue))
      (bind _output_get (Variables|Default|SetLootItems _returnvalue_2))
      (Variables|Default|SetLootRotations (CallFunction|GetLootRotations _output_get))
      (Variables|Default|SetSpawnLootCount 0)
      (bind _returnvalue_3 (Utilities|Time|SetTimerbyEvent (delegate Custom|SpawnLootItem) 0.1 true))
      (Variables|Default|SetLootTimer _returnvalue_3)
      (CallFunction|SpawnLootItem))))

(fn ConstructionScript)

(fn GetLootRotations
  (params (TargetArray :type Array%20of%20Loot%20Item%20Structures))
  (return (Class|RPGAbilitySystemLibrary|EvenlySpacedRotators (Transformation|GetActorForwardVector) (Math|Vector|VectorUp) 3.6e+02 (Utilities|Array|Length TargetArray))))

(fn GetLootTransform
  (params (Dimension%201 :type Integer))
  (bind _returnvalue (Transformation|GetActorLocation))
  (bind _maxspawndistance (Variables|Default|GetMaxSpawnDistance))
  (bind _lootrotations (Variables|Default|GetLootRotations))
  (bind _minspawndistance (Variables|Default|GetMinSpawnDistance))
  (bind _returnvalue_2 (Math|Random|RandomFloatinRange _minspawndistance _maxspawndistance))
  (bind _output (Utilities|Array|Get(acopy) _lootrotations Dimension%201))
  (bind _returnvalue_3 (Math|Vector|GetForwardVector _output))
  (bind _returnvalue_4 (* _returnvalue_3 _returnvalue_2))
  (bind _returnvalue_5 (+ _returnvalue_4 _returnvalue))
  (return (Math|Transform|MakeTransform (Math|Vector|MakeVector (.x _returnvalue_5) (.y _returnvalue_5) 5e+01) _output)))

(fn UpdateLootLevel
  (params (Object :type Object%20Object%20Reference) (Condition :type Boolean))
  (if Condition
    (bind _asrpgeffect_actor (Utilities|Casting|CastToRPGEffectActor Object))
    (Utilities|IsValid _asrpgeffect_actor
      (:Is%20Valid
        (bind _returnvalue (Class|CombatInterface|GetPlayerLevel))
        (Variables|/Script/RPG.RPGEffectActor|SetActorLevel _asrpgeffect_actor (Math|Conversions|ToFloat(Integer) _returnvalue))))))