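; BP_Beacon is a checkpoint beacon that activates once, with a glow, when an actor reaches it.
; A Sphere overlap by an actor implementing PlayerInterface sets the Reached flag and calls HandleGlowEffects, which is defined outside this graph.
; The CheckpointReached event receives a dynamic material instance and plays a timeline that drives its GlowControl scalar parameter.
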(event OnComponentBeginOverlap(Sphere)
  (params (OverlappedComponent :type Primitive%20Component%20Object%20Reference) (OtherActor :type Actor%20Object%20Reference) (OtherComp :type Primitive%20Component%20Object%20Reference) (OtherBodyIndex :type Integer) (bFromSweep :type Boolean) (SweepResult :type Hit%20Result%20Structure%20%28by%20ref%29))
  (if (Utilities|DoesObjectImplementInterface OtherActor "/Script/RPG.PlayerInterface")
    (if (not (Variables|Default|GetbReached))
      (Variables|Default|SetbReached true)
      (Class|CheckPoint|HandleGlowEffects))))

(event EventBeginPlay)

(event EventTick
  (params (DeltaSeconds :type Float%20%28single-precision%29)))

(event EventCheckpointReached
  (params (DynamicMaterialInstance :type Material%20Instance%20Dynamic%20Object%20Reference))
  (Variables|Default|SetDynamic%20Material%20Instance DynamicMaterialInstance)
  (bind _glowtrack (Timeline|时间轴 Play)
    (:Update
      (Rendering|Material|SetScalarParameterValue (Variables|Default|GetDynamic%20Material%20Instance) "GlowControl" _glowtrack :!class /Script/Engine.MaterialInstanceDynamic))))

(fn ConstructionScript)