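; BP_FadeActor is a static mesh actor that fades out and back in, automatically demonstrating this on BeginPlay with a two-second delay.
; Construction caches original materials and builds dynamic instances from a set of fade materials.
; FadeOut and FadeIn swap those in, then play or reverse a timeline driving their "Fade" parameter.
; Finishing forward ignores the Visibility channel; finishing backward restores original materials and blocking.
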(event Custom|FadeOut
  (CallFunction|SetMaterialstoDynamicInstance)
  (bind (_direction _fade) (Timeline|时间轴 Play)
    (:Update
      (for _array_element (Variables|Default|GetDynamicMaterialInstance)
        (Rendering|Material|SetScalarParameterValue _array_element "Fade" _fade :!class /Script/Engine.MaterialInstanceDynamic)))
    (:Finished
      (CallFunction|FadeFinished _direction))))

(event Custom|FadeIn
  (CallFunction|SetMaterialstoDynamicInstance)
  (bind (_direction _fade) (Timeline|时间轴 Reverse)
    (:Update
      (for _array_element (Variables|Default|GetDynamicMaterialInstance)
        (Rendering|Material|SetScalarParameterValue _array_element "Fade" _fade :!class /Script/Engine.MaterialInstanceDynamic)))
    (:Finished
      (CallFunction|FadeFinished _direction))))

(event EventBeginPlay
  (CallFunction|FadeOut)
  (Utilities|FlowControl|Delay 2.0)
  (CallFunction|Fadein))

(event Collision|EventActorBeginOverlap
  (params (OtherActor :type Actor%20Object%20Reference)))

(event EventTick
  (params (DeltaSeconds :type Float%20%28single-precision%29)))

(fn ConstructionScript
  (Variables|Default|SetOriginalMaterials (Rendering|Material|GetMaterials (Variables|Default|GetStaticMesh)))
  (Utilities|Array|Clear (Variables|Default|GetDynamicMaterialInstance))
  (for _array_element (Variables|Default|GetFadeMaterialsInstance)
    (bind _returnvalue (Rendering|Material|CreateDynamicMaterialInstance _array_element "None" "None" :!class /Script/Engine.KismetMaterialLibrary))
    (Utilities|Array|AddUnique (Variables|Default|GetDynamicMaterialInstance) _returnvalue)))

(fn SetMaterialstoDynamicInstance
  (for (_array_element _array_index) (Variables|Default|GetDynamicMaterialInstance)
    (Rendering|Material|SetMaterial (Variables|Default|GetStaticMesh) _array_index _array_element)))

(fn ResetMaterials
  (for (_array_element _array_index) (Variables|Default|GetOriginalMaterials)
    (Rendering|Material|SetMaterial (Variables|Default|GetStaticMesh) _array_index _array_element)))

(fn FadeFinished
  (params (Selection :type ETimelineDirection%20Enum :default "Forward"))
  (bind _staticmesh (Variables|Default|GetStaticMesh))
  (switch Utilities|FlowControl|Switch|SwitchonETimelineDirection Selection
    (:Forward
      (Collision|SetCollisionResponsetoChannel _staticmesh "ECC_Visibility" "ECR_Ignore"))
    (:Backward
      (CallFunction|ResetMaterials)
      (Collision|SetCollisionResponsetoChannel _staticmesh "ECC_Visibility" "ECR_Block"))))